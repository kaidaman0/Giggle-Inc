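; BP_TheWorld is a "Za Warudo" enemy drawn as a plane that yaws to face the player camera.
; A second after BeginPlay, a FlipFlop sends it toward the last sensed pawn's location, then on arrival to a random reachable point, where it spawns a burst effect and destroys itself.
; PawnSensing supplies the chase target, and capsule overlap with the player plays a sound behind a DoOnce cooldown.
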(event `self.ReceiveTick`
  (params (DeltaSeconds :type "Float (single-precision)"))
  (bind (_returnvalue_roll _returnvalue_pitch _returnvalue_yaw) (`KismetMathLibrary.BreakRotator` (`KismetMathLibrary.FindLookAtRotation` (`SceneComponent.K2_GetComponentLocation` (`self.Plane`)) (`PlayerCameraManager.GetCameraLocation` (`GameplayStatics.GetPlayerCameraManager` 0)))))
  ; Lookat
  (`SceneComponent.K2_SetWorldRotation` (`self.Plane`) (`KismetMathLibrary.MakeRotator` -270.0 0.0 (+ _returnvalue_yaw -90.0)) false false))

(event `self.ReceiveBeginPlay`
  ; Start
  (`KismetSystemLibrary.Delay` 1.0)
  (`self.Timer`))

(event `Timer`
  ; Timer
  (`/Engine/EditorBlueprintResources/StandardMacros.FlipFlop`
    (:`A`
      (`self.Chase`))
    (:`B`
      (`self.Random`))))

(event `Chase`
  ; Chase
  (`|AIMoveTo` self (`self.K2_GetActorLocation` (`self.PlayerPawnSensed`)) null 10.0
    (:`OnSuccess`
      (`self.Timer`))))

(event `Random`
  ; Random
  (`|AIMoveTo` self (`NavigationSystemV1.K2_GetRandomReachablePointInRadius` (`self.K2_GetActorLocation` self) 10000.0 null "/Script/AIModule.NavFilter_AIControllerDefault") null
    (:`OnSuccess`
      (`NiagaraFunctionLibrary.SpawnSystemAtLocation` "/Game/AI/Enemies/ZaWarudo/Burst.Burst" (`SceneComponent.K2_GetComponentLocation` (`self.CapsuleComponent`)))
      (`self.K2_DestroyActor`))))

(event `self.PawnSensing.OnSeePawn`
  (params (Pawn :type "Pawn Object Reference"))
  (set `self.PlayerPawnSensed` Pawn)
  (set `self.CanSeePlayer?` true))

(event `self.Capsule.OnComponentBeginOverlap`
  (params (OverlappedComponent :type "PrimitiveComponent Object Reference") (OtherActor :type "Actor Object Reference") (OtherComp :type "PrimitiveComponent Object Reference") (OtherBodyIndex :type Integer) (bFromSweep :type Boolean) (SweepResult :type "HitResult Structure (by ref)"))
  (if (`self.ActorHasTag` OtherActor "Player")
    (`/Engine/EditorBlueprintResources/StandardMacros.DoOnce` false :!label _label
      (:`Completed`
        (`GameplayStatics.PlaySound2D` "/Game/AI/Enemies/ZaWarudo/Za_Warudo_-_Sound_Effect.Za_Warudo_-_Sound_Effect" 1.0 1.0 0.0 null null)
        (`KismetSystemLibrary.Delay` 5.0)
        (goto _label :!via `Reset`)))))

(fn `UserConstructionScript`)